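; Ceiling lamp actor that holds an on/off flag for its point light and starts with the flag off.
; TurnLightsOn and TurnLightsOff only set LightValue; BeginPlay calls TurnLightsOff.
; While LightValue is true, Tick toggles the PointLight's visibility every frame, making it flicker rather than stay lit.
; When the flag is false, visibility is left in whatever state it was last in.
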(event EventBeginPlay
  (CallFunction|TurnLightsOff))

(event Collision|EventActorBeginOverlap
  (params (OtherActor :type Actor%20Object%20Reference)))

(event EventTick
  (params (DeltaSeconds :type Float%20%28single-precision%29))
  (if (Variables|Default|GetLightValue)
    (Rendering|ToggleVisibility (Variables|Default|GetPointLight) false)))

(fn ConstructionScript)

(fn TurnLightsOff
  (Variables|Default|SetLightValue (Class|KismetSystemLibrary|MakeLiteralBool false)))

(fn TurnLightson
  (Variables|Default|SetLightValue (Class|KismetSystemLibrary|MakeLiteralBool true)))